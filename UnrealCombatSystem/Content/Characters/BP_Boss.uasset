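; BP_Boss is a boss character that runs the BT_BOSS behavior tree and shows a lock-on widget while selected.
; Damage reduces health in its stats component, whose delegates update the boss health bar and, at zero health, trigger death handling and remove the bar.
; Pawn sensing passes seen pawns to DetectPawn against the player and creates the health bar once, on the first sighting of any pawn.
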(event `self.ReceiveBeginPlay`
  (`AIController.RunBehaviorTree` (`AIBlueprintHelperLibrary.GetAIController` self) "/Game/Characters/AI/BT_BOSS.BT_BOSS"))

(event `self.OnSelect`
  (`SceneComponent.SetVisibility` (`self.LockOnWidget`) true false))

(event `self.OnDeselect`
  (`SceneComponent.SetVisibility` (`self.LockOnWidget`) false false))

(event `self.ReceiveAnyDamage`
  (params (Damage :type "Float (single-precision)") (DamageType :type "DamageType Object Reference") (InstigatedBy :type "Controller Object Reference") (DamageCauser :type "Actor Object Reference"))
  (`StatsComponent.ReduceHealth` (`self.m_statsComponent`) Damage null))

(event `self.PawnSensing.OnSeePawn`
  (params (Pawn :type "Pawn Object Reference"))
  (`self.DetectPawn` Pawn (`GameplayStatics.GetPlayerPawn` 0))
  (`/Engine/EditorBlueprintResources/StandardMacros.DoOnce` false
    (:`Completed`
      (bind _returnvalue (`|CreateWidget` "/Game/UI/WBP_Boss.WBP_Boss_C"))
      (bind _output_get (set `self.BossUI` _returnvalue))
      (`UserWidget.AddToViewport` _output_get 0)
      (`/Game/UI/WBP_Boss.Set Health` (`self.BossUI`) (`StatsComponent.GetStatPercentage` (`self.m_statsComponent`) "Health" "MaxHealth")))))

(event `self.m_statsComponent.m_OnHealthPercentUpdateDelegate`
  (params (Percentage :type "Float (single-precision)"))
  (`/Game/UI/WBP_Boss.Set Health` (`self.BossUI`) Percentage))

(event `self.m_statsComponent.m_onZeroHealthDelegate`
  (`self.HandleDeath`)
  (`Widget.RemoveFromParent` (`self.BossUI`)))

(fn `UserConstructionScript`)